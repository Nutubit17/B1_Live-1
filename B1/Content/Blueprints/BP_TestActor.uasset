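; BP_TestActor is a test actor that prints debug strings when play begins.
; BeginPlay calls PrintS, which uses a sequence to print a greeting if Hp is at or above a threshold, then prints each index of a short counting loop.
; A separate TestFunc returns the sum of its two inputs but is not called here, and Tick and the construction script are empty.
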(event EventBeginPlay
  (CallFunction|PrintS))

(event EventTick
  (params (DeltaSeconds :type Float%20%28single-precision%29)))

(fn ConstructionScript)

(fn TestFunc
  (params (A :type Integer) (B :type Integer))
  (return (+ A B)))

(fn PrintS
  (Utilities|FlowControl|Sequence
    (:then_0
      (if (>= (Variables|Default|GetHp) 100)
        (Development|PrintString "Hello")))
    (:then_1
      (for _index (range 1 10)
        (Development|PrintString (Utilities|String|ToString(Integer) _index))))))